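; BP_EnermySpawner is an actor that repeatedly spawns waves of an enemy class at its own transform.
; BeginPlay calls the SpawnEnermy event, which spawns LastIndex copies of the Enermy class in a loop at the same transform.
; After a SpawnDelay wait, the event calls itself with the spawner's current transform, repeating with no stop condition or cap on live enemies.
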(event Custom|SpawnEnermy
  (params (Enermy :type Actor%20Class%20Reference) (SpawnTransform :type Transform) (LastIndex :type Integer))
  (for _index (range 0 (- LastIndex 1))
    (Game|SpawnActorfromClass Enermy SpawnTransform "Undefined" 0 0))
  (Utilities|FlowControl|Delay (Variables|Default|GetSpawnDelay))
  (CallFunction|SpawnEnermy (Variables|Default|GetEnermy) (Transformation|GetActorTransform) (Variables|Default|GetLast%20Index)))

(event EventBeginPlay
  (CallFunction|SpawnEnermy (Variables|Default|GetEnermy) (Transformation|GetActorTransform) (Variables|Default|GetLast%20Index)))

(fn ConstructionScript)