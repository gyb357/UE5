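; BP_Enermy is an enemy pawn that chases the player and takes damage from projectiles.
; When PawnSensing sees any pawn, it sets IsSee, which is never cleared here, and runs AIMoveTo toward player character 0.
; Each BP_Projectile hit lowers Health by one, but destruction only happens on a hit that finds Health already below zero.
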(event OnSeePawn(PawnSensing)
  (params (Pawn :type Pawn%20Object%20Reference))
  ;[1 1 1] PawnSensing
  (Variables|Default|SetisSee true)
  (CallFunction|FollowPlayer))

(event Custom|FollowPlayer
  ;[1 1 1] FollowPlayer
  (if (Variables|Default|GetisSee)
    (AI|AIMoveTo self "0, 0, 0" (Game|GetPlayerCharacter 0) 5.0 false)))

(event Collision|EventHit
  (params (MyComp :type Primitive%20Component%20Object%20Reference) (Other :type Actor%20Object%20Reference) (OtherComp :type Primitive%20Component%20Object%20Reference) (bSelfMoved :type Boolean) (HitLocation :type Vector :default "0, 0, 0") (HitNormal :type Vector :default "0, 0, 0") (NormalImpulse :type Vector :default "0, 0, 0") (Hit :type Hit%20Result%20Structure%20%28by%20ref%29))
  ;[1 1 1] Hit
  (Utilities|Casting|CastToBP_Projectile Other)
  (if (< (Variables|Default|GetHealth) 0.0)
    (Actor|DestroyActor)
    (else
      (Variables|Default|SetHealth (- (Variables|Default|GetHealth) 1.0)))))

(fn ConstructionScript)